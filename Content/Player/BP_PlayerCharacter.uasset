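; Player character Blueprint that creates the HUD widgets and drives sword combat and a toggleable lantern.
; Stamina-gated attacks (alternating swings, thrust) and a state-machine-backed block use timelines to procedurally animate the RightHand child actor, which Tick eases back to rest.
; Timeline tracks toggle CanDoAction to lock input, and sword overlaps damage HealthComponents while it is false.
; Looping timers ease lantern intensity between zero and current fuel.
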(event OnComponentBeginOverlap(SwordCollision)
  (params (OverlappedComponent :type Primitive%20Component%20Object%20Reference) (OtherActor :type Actor%20Object%20Reference) (OtherComp :type Primitive%20Component%20Object%20Reference) (OtherBodyIndex :type Integer) (bFromSweep :type Boolean) (SweepResult :type Hit%20Result%20Structure%20%28by%20ref%29))
  (bind _returnvalue (Actor|GetComponentbyClass OtherActor "/Script/ProjectDarkCave.HealthComponent"))
  (if (and (Utilities|IsValid _returnvalue) (not (Variables|Default|GetbCanDoAction)))
    (Class|HealthComponent|TakeDamage _returnvalue 12.5))
  (Development|PrintString (Utilities|GetDisplayName OtherActor)))

(event Custom|TurnLightOff
  (bind _playerlightcomponent (Variables|Default|GetPlayerLightComponent))
  (bind _intensity (Variables|/Script/Engine.LightComponentBase|GetIntensity _playerlightcomponent))
  (bind _result (Math|Interpolation|Ease "EaseInOut" 0.2 _intensity 0.0 2.0))
  ;[0.15 0.15 0.15 0.5] Use Light
  (if (<= (Variables|/Script/Engine.LightComponentBase|GetIntensity (Variables|Default|GetPlayerLightComponent)) 0.0)
    (Utilities|Time|ClearandInvalidateTimerbyHandle (Variables|Default|GetTurnLightOffTimerHandle))
    (Variables|Default|SetbLightIsOn false)
    (Variables|Default|SetbLightIsTransitioning false)
    (elif (< _result 0.01)
      (Rendering|Components|Light|SetIntensity _playerlightcomponent 0.0)
      (else
        (Rendering|Components|Light|SetIntensity _playerlightcomponent _result)))))

(event Custom|TurnLightOn
  (bind _playerlightcomponent (Variables|Default|GetPlayerLightComponent))
  (bind _currentlightfuel (Variables|Default|GetcurrentLightFuel))
  (bind _intensity (Variables|/Script/Engine.LightComponentBase|GetIntensity _playerlightcomponent))
  (bind _result (Math|Interpolation|Ease "EaseInOut" 0.2 _intensity _currentlightfuel 2.0))
  ;[0.15 0.15 0.15 0.5] Use Light
  (if (>= (Variables|/Script/Engine.LightComponentBase|GetIntensity (Variables|Default|GetPlayerLightComponent)) (- (Variables|Default|GetcurrentLightFuel) 0.1))
    (Utilities|Time|ClearandInvalidateTimerbyHandle (Variables|Default|GetTurnLightOnTimerHandle))
    (Variables|Default|SetbLightIsOn true)
    (Variables|Default|SetbLightIsTransitioning false)
    (elif (> _result (- _currentlightfuel 0.1))
      (Rendering|Components|Light|SetIntensity _playerlightcomponent _currentlightfuel)
      (else
        (Rendering|Components|Light|SetIntensity _playerlightcomponent _result)))))

(event Input|EnhancedActionEvents|EnhancedInputActionIA_UseRightHand
  (params (ActionValue :type Boolean) (ElapsedSeconds :type Float%20%28double-precision%29) (TriggeredSeconds :type Float%20%28double-precision%29) (InputAction :type Input%20Action%20Object%20Reference :default "/Game/Input/IA_UseRightHand.IA_UseRightHand"))
  ;[0.15 0.15 0.15 0.5] Attack Animation Logic
  (:Started
    (bind _returnvalue (Class|PlayerStateMachine|IsBlocking (Variables|Default|GetPlayerStateMachine)))
    (if (and (not _returnvalue) (Variables|Default|GetbCanDoAction))
      (bind _returnvalue_2 (Class|PlayerHandler|DecreaseStamina (Variables|Default|GetstaminaAttackCost)))
      (if _returnvalue_2
        (Variables|Default|SetStartedResetRightHand false)
        (if (Variables|Default|GetbIsAttackingRight)
          (Variables|Default|SetbIsAttackingRight false)
          (bind (_direction _attack_location _attack_rotation _can_do_action) (Timeline|AttackLeft PlayFromStart)
            (:Update
              (CallFunction|PlayandEaseAnimation (Variables|Default|GetRightHand) _attack_location (.x _attack_rotation) (.y _attack_rotation) (.z _attack_rotation) 0.3 0.5)
              (Math|Float|CompareFloat _can_do_action 1.0
                (:>
                  (Variables|Default|SetbCanDoAction true :!label _label)
                  (bind (_direction_2 _attack_location_2 _attack_rotation_2 _can_do_action_2) (Timeline|Attack Stop)
                    (:Update
                      (CallFunction|PlayandEaseAnimation (Variables|Default|GetRightHand) _attack_location_2 (.x _attack_rotation_2) (.y _attack_rotation_2) (.z _attack_rotation_2) 0.3 0.5)
                      (Math|Float|CompareFloat _can_do_action_2 1.0
                        (:>
                          (Variables|Default|SetbCanDoAction true :!label _label_2)
                          (Timeline|AttackLeft Stop))
                        (:==
                          (goto _label_2))
                        (:<
                          (Variables|Default|SetbCanDoAction false)
                          (Timeline|AttackLeft Stop))))
                    (:Finished
                      (Variables|Default|SetStartedResetRightHand true :!label _label_3)
                      (Variables|Default|SetbIsAttackingRight false))))
                (:==
                  (goto _label))
                (:<
                  (Variables|Default|SetbCanDoAction false)
                  (Timeline|Attack Stop))))
            (:Finished
              (goto _label_3)))
          (else
            (Variables|Default|SetbIsAttackingRight true)
            (Timeline|Attack PlayFromStart)))))))

(event Input|EnhancedActionEvents|EnhancedInputActionIA_UseSecondaryAction
  (params (ActionValue :type Boolean) (ElapsedSeconds :type Float%20%28double-precision%29) (TriggeredSeconds :type Float%20%28double-precision%29) (InputAction :type Input%20Action%20Object%20Reference :default "/Game/Input/IA_UseSecondaryAction.IA_UseSecondaryAction"))
  (bind _playerstatemachine (Variables|Default|GetPlayerStateMachine))
  ;[0.15 0.15 0.15 0.5] Attack Animation Logic
  (:Triggered
    (if (Variables|Default|GetbCanDoAction)
      (Class|PlayerStateMachine|SetStateBlocking _playerstatemachine true)
      (Variables|Default|SetStartedResetRightHand false)
      (bind (_direction _block_location _block_rotation) (Timeline|Block PlayFromStart)
        (:Update
          (CallFunction|PlayandEaseAnimation (Variables|Default|GetRightHand) _block_location (.x _block_rotation) (.y _block_rotation) (.z _block_rotation) 0.15 0.2)
          (Variables|Default|SetbIsAttackingRight false)
          (Utilities|FlowControl|Sequence
            (:then_0
              (bind (_direction_2 _attack_location _attack_rotation _can_do_action) (Timeline|Attack Stop)
                (:Update
                  (CallFunction|PlayandEaseAnimation (Variables|Default|GetRightHand) _attack_location (.x _attack_rotation) (.y _attack_rotation) (.z _attack_rotation) 0.3 0.5)
                  (Math|Float|CompareFloat _can_do_action 1.0
                    (:>
                      (Variables|Default|SetbCanDoAction true :!label _label)
                      (bind (_direction_3 _attack_location_2 _attack_rotation_2 _can_do_action_2) (Timeline|AttackLeft Stop)
                        (:Update
                          (CallFunction|PlayandEaseAnimation (Variables|Default|GetRightHand) _attack_location_2 (.x _attack_rotation_2) (.y _attack_rotation_2) (.z _attack_rotation_2) 0.3 0.5)
                          (Math|Float|CompareFloat _can_do_action_2 1.0
                            (:>
                              (Variables|Default|SetbCanDoAction true :!label _label_2)
                              (Timeline|Attack Stop))
                            (:==
                              (goto _label_2))
                            (:<
                              (Variables|Default|SetbCanDoAction false)
                              (Timeline|Attack Stop))))
                        (:Finished
                          (Variables|Default|SetStartedResetRightHand true :!label _label_3)
                          (Variables|Default|SetbIsAttackingRight false))))
                    (:==
                      (goto _label))
                    (:<
                      (Variables|Default|SetbCanDoAction false)
                      (Timeline|AttackLeft Stop))))
                (:Finished
                  (goto _label_3))))
            (:then_1
              (Timeline|AttackLeft Stop)))))))
  (:Completed
    (Class|PlayerStateMachine|SetStateBlocking _playerstatemachine false)
    (Utilities|FlowControl|Sequence
      (:then_0
        (Timeline|Block Stop))
      (:then_1
        (goto _label_3)))))

(event Input|EnhancedActionEvents|EnhancedInputActionIA_UseBlockAttack
  (params (ActionValue :type Boolean) (ElapsedSeconds :type Float%20%28double-precision%29) (TriggeredSeconds :type Float%20%28double-precision%29) (InputAction :type Input%20Action%20Object%20Reference :default "/Game/Input/IA_UseBlockAttack.IA_UseBlockAttack"))
  ;[0.15 0.15 0.15 0.5] Attack Animation Logic
  (:Started
    (if (Variables|Default|GetbCanDoAction)
      (bind _returnvalue (Class|PlayerHandler|DecreaseStamina (Variables|Default|GetstaminaAttackCost)))
      (if _returnvalue
        (bind (_direction _attack_location _attack_rotation _can_do_action) (Timeline|AttackThrust PlayFromStart)
          (:Update
            (CallFunction|PlayandEaseAnimation (Variables|Default|GetRightHand) _attack_location (.x _attack_rotation) (.y _attack_rotation) (.z _attack_rotation) 0.3 0.3)
            (Math|Float|CompareFloat _can_do_action 1.0
              (:>
                (Variables|Default|SetbCanDoAction true :!label _label))
              (:==
                (goto _label))
              (:<
                (Variables|Default|SetbCanDoAction false)))))))))

(event Input|EnhancedActionEvents|EnhancedInputActionIA_UseLight
  (params (ActionValue :type Boolean) (ElapsedSeconds :type Float%20%28double-precision%29) (TriggeredSeconds :type Float%20%28double-precision%29) (InputAction :type Input%20Action%20Object%20Reference :default "/Game/Input/IA_UseLight.IA_UseLight"))
  ;[0.15 0.15 0.15 0.5] Use Light
  (:Started
    (Variables|Default|SetbLightIsTransitioning true)
    (if (Variables|Default|GetbLightIsOn)
      (bind _returnvalue (Utilities|Time|SetTimerbyFunctionName 0 "TurnLightOff" 0.01 true))
      (Variables|Default|SetTurnLightOffTimerHandle _returnvalue)
      (else
        (bind _returnvalue_2 (Utilities|Time|SetTimerbyFunctionName 0 "TurnLightOn" 0.01 true))
        (Variables|Default|SetTurnLightOnTimerHandle _returnvalue_2)))))

(event EventBeginPlay
  (bind _righthand (Variables|Default|GetRightHand))
  (Utilities|FlowControl|Sequence
    (:then_0
      (bind _returnvalue (UserInterface|CreateWidget "/Game/WBP_StaminaBar.WBP_StaminaBar_C"))
      (UserInterface|Viewport|AddtoViewport _returnvalue 0)
      (bind _returnvalue_2 (UserInterface|CreateWidget "/Game/WBP_LightFuelBar.WBP_LightFuelBar_C"))
      (UserInterface|Viewport|AddtoViewport _returnvalue_2 0)
      (bind _returnvalue_3 (UserInterface|CreateWidget "/Game/WBP_Crosshair.WBP_Crosshair_C"))
      (UserInterface|Viewport|AddtoViewport _returnvalue_3 0)
      (bind _returnvalue_4 (UserInterface|CreateWidget "/Game/WBP_Inventory.WBP_Inventory_C"))
      (UserInterface|Viewport|AddtoViewport _returnvalue_4 0)
      (bind _returnvalue_5 (UserInterface|CreateWidget "/Game/WBP_HealthBar.WBP_HealthBar_C"))
      (UserInterface|Viewport|AddtoViewport _returnvalue_5 0))
    (:then_1
      (Variables|Default|SetDefaultRightHandPos (Variables|/Script/Engine.SceneComponent|GetRelativeLocation _righthand))
      (Variables|Default|SetDefaultRightHandRotation (Variables|/Script/Engine.SceneComponent|GetRelativeRotation _righthand)))
    (:then_2
      (bind _output_get (Variables|Default|SetPlayerLightComponent (Actor|GetComponentbyClass (Variables|/Script/Engine.ChildActorComponent|GetChildActor (Variables|Default|GetBPP_Level_Lantern)) "/Script/Engine.PointLightComponent")))
      (Rendering|Components|Light|SetIntensity _output_get (Variables|Default|GetmaxLightFuel)))))

(event EventTick
  (params (DeltaSeconds :type Float%20%28single-precision%29))
  (bind _defaultrighthandpos (Variables|Default|GetDefaultRightHandPos))
  (bind _defaultrighthandrotation (Variables|Default|GetDefaultRightHandRotation))
  (bind _righthand (Variables|Default|GetRightHand))
  (bind _relativelocation (Variables|/Script/Engine.SceneComponent|GetRelativeLocation _righthand))
  (bind _relativerotation (Variables|/Script/Engine.SceneComponent|GetRelativeRotation _righthand))
  (Utilities|FlowControl|Sequence
    (:then_0
      (if (and (Variables|Default|GetStartedResetRightHand) (Variables|Default|GetbCanDoAction))
        (Transformation|SetRelativeLocationAndRotation _righthand (Math|Interpolation|VInterpTo _relativelocation _defaultrighthandpos 0.3 0.3) (Math|Interpolation|Ease "EaseInOut" 0.2 _relativerotation _defaultrighthandrotation true) false false)
        (if (and (Utilities|Operators|EqualEqual _relativelocation _defaultrighthandpos 0.0) (Utilities|Operators|EqualEqual _relativerotation _defaultrighthandrotation 0.0))
          (Variables|Default|SetStartedResetRightHand false))))))

(fn ConstructionScript)